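; Road actor that lets the player hold an input to be carried along it, and sends them back if they fail.
; Entering Box shows a HoldVisual widget; holding IA_Hold past a short threshold runs a timeline lerping the character toward the Scene component.
; Releasing stops movement; releasing inside Box2, or entering it without holding, fades the camera and teleports the player to the Teleport component.
; Overlapping EndOfRoad disables the hold interaction.
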(event `WidgetLOL`
  ;[1 1 1] Create hold visual
  (bind _returnvalue (`|CreateWidget` "/Game/UI/HoldVisual.HoldVisual_C"))
  (`UserWidget.AddToViewport` _returnvalue 0))

(event `self.Box.OnComponentBeginOverlap`
  (params (OverlappedComponent :type "PrimitiveComponent Object Reference") (OtherActor :type "Actor Object Reference") (OtherComp :type "PrimitiveComponent Object Reference") (OtherBodyIndex :type Integer) (bFromSweep :type Boolean) (SweepResult :type "HitResult Structure (by ref)"))
  ;[1 1 1] Player near road
  (if (== OtherActor (`GameplayStatics.GetPlayerCharacter` 0))
    (set `self.PlayerNearRoad` true)
    (`self.WidgetLOL`)))

(event `self.EndOfRoad.OnComponentBeginOverlap`
  (params (OverlappedComponent :type "PrimitiveComponent Object Reference") (OtherActor :type "Actor Object Reference") (OtherComp :type "PrimitiveComponent Object Reference") (OtherBodyIndex :type Integer) (bFromSweep :type Boolean) (SweepResult :type "HitResult Structure (by ref)"))
  ;[1 1 1] Player not near road
  (if (== OtherActor (`GameplayStatics.GetPlayerCharacter` 0))
    (set `self.PlayerNearRoad` false)))

(event `EnhancedInput|/Game/FirstPerson/Input/Actions/IA_Hold`
  (params (ActionValue :type Boolean) (ElapsedSeconds :type "Float (double-precision)") (TriggeredSeconds :type "Float (double-precision)") (InputAction :type "InputAction Object Reference" :default "/Game/FirstPerson/Input/Actions/IA_Hold.IA_Hold"))
  (bind _returnvalue (`GameplayStatics.GetPlayerCameraManager` 0))
  (bind _returnvalue_2 (`GameplayStatics.GetPlayerCharacter` 0))
  ;[1 1 1] Player move
  (:`Ongoing`
    (if (`self.PlayerNearRoad`)
      (`TimelineComponent.SetPlayRate` (`self.Player_Move`) 0.09)
      (if (>= ElapsedSeconds 0.9)
        (set `self.Holding_Space` true)
        (bind (_direction _move) (`Timeline|Player_Move` :!via `PlayFromStart` :!label _label)
          (:`Update`
            (`self.K2_SetActorLocation` _returnvalue_2 (`KismetMathLibrary.VLerp` (`self.K2_GetActorLocation` _returnvalue_2) (`SceneComponent.K2_GetComponentLocation` (`self.Scene`)) _move) false false))))))
  (:`Completed`
    (`|ExecutionSequence`
      (:`then_0`
        (goto _label :!via `Stop`))
      (:`then_1`
        (if (`self.OnRoad`)
          ;[1 1 1] Camera fade and reappear
          (`PlayerCameraManager.StartCameraFade` :`self` _returnvalue :`ToAlpha` 1.0 :`Duration` 0.5 :`bHoldWhenFinished` true :!label _label_2)
          (`KismetSystemLibrary.Delay` 0.5)
          (`self.K2_SetActorLocation` (`GameplayStatics.GetPlayerCharacter` 0) (`SceneComponent.K2_GetComponentLocation` (`self.Teleport`)) false true)
          (`KismetSystemLibrary.Delay` 1.0)
          (`PlayerCameraManager.StartCameraFade` :`self` _returnvalue :`FromAlpha` 1.0 :`Duration` 2.0 :`bHoldWhenFinished` true))))))

(event `self.Box 2.OnComponentBeginOverlap`
  (params (OverlappedComponent :type "PrimitiveComponent Object Reference") (OtherActor :type "Actor Object Reference") (OtherComp :type "PrimitiveComponent Object Reference") (OtherBodyIndex :type Integer) (bFromSweep :type Boolean) (SweepResult :type "HitResult Structure (by ref)"))
  ;[1 1 1] On Road? Checkers
  (if (== OtherActor (`GameplayStatics.GetPlayerCharacter` 0))
    (if (`self.Holding_Space`)
      (set `self.OnRoad` true)
      (else
        (goto _label_2)))))

(event `self.Box 2.OnComponentEndOverlap`
  (params (OverlappedComponent :type "PrimitiveComponent Object Reference") (OtherActor :type "Actor Object Reference") (OtherComp :type "PrimitiveComponent Object Reference") (OtherBodyIndex :type Integer))
  ;[1 1 1] On Road? Checkers
  (if (== OtherActor (`GameplayStatics.GetPlayerCharacter` 0))
    (set `self.OnRoad` false)
    (`Widget.RemoveFromParent` (stale `WidgetLOL` _returnvalue) :!label _label_3)))

(event `self.Box.OnComponentEndOverlap`
  (params (OverlappedComponent :type "PrimitiveComponent Object Reference") (OtherActor :type "Actor Object Reference") (OtherComp :type "PrimitiveComponent Object Reference") (OtherBodyIndex :type Integer))
  ;[1 1 1] Player near road
  (if (== OtherActor (`GameplayStatics.GetPlayerCharacter` 0))
    (set `self.PlayerNearRoad` false)
    (goto _label_3)))

(fn `UserConstructionScript`)