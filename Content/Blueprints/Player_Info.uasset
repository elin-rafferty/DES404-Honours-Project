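; Player Info is an actor that persists the player's music and narrative volume settings through BP_Player_Save_Game.
; On BeginPlay or a Load call it loads the slot asynchronously and applies both volumes as sound mix class overrides, or saves a fresh default object if none exists.
; SaveGame reloads the existing slot, copies the current values into it and writes it back asynchronously.
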(event `Load`
  (bind _returnvalue (`GameplayStatics.DoesSaveGameExist` (`self.Slot Name`) :!label _label))
  (if _returnvalue
    (bind _savegame (`AsyncActionHandleSaveGame.AsyncLoadGameFromSlot` (`self.Slot Name`))
      (:`Completed`
        (`/Engine/EditorBlueprintResources/StandardMacros.IsValid` _savegame
          (:`Is Valid`
            (bind _asbp_player_save_game (cast `/Game/Blueprints/BP_Player_Save_Game` _savegame))
            (`/Engine/EditorBlueprintResources/StandardMacros.IsValid` _asbp_player_save_game
              (:`Is Valid`
                (`self.Load Info` _asbp_player_save_game)
                (`KismetSystemLibrary.PrintString` "Loaded")))))))
    (else
      (bind _returnvalue_2 (`GameplayStatics.CreateSaveGameObject` "/Game/Blueprints/BP_Player_Save_Game.BP_Player_Save_Game_C"))
      (bind _output_get (set `self.Bp_Player_Save_game` _returnvalue_2))
      (`AsyncActionHandleSaveGame.AsyncSaveGameToSlot` _output_get (`self.Slot Name`)
        (:`Completed`
          (`KismetSystemLibrary.PrintString` "New Save Game"))))))

(event `self.ReceiveBeginPlay`
  (goto _label))

(event `Save Game`
  (bind _savegame (`AsyncActionHandleSaveGame.AsyncLoadGameFromSlot` (`self.Slot Name`))
    (:`Completed`
      (`/Engine/EditorBlueprintResources/StandardMacros.IsValid` _savegame
        (:`Is Valid`
          (bind _asbp_player_save_game (cast `/Game/Blueprints/BP_Player_Save_Game` _savegame))
          (`self.Save_Info` _asbp_player_save_game)
          (`AsyncActionHandleSaveGame.AsyncSaveGameToSlot` _asbp_player_save_game (`self.Slot Name`)
            (:`Completed`
              (`KismetSystemLibrary.PrintString` "Saved"))))))))

(fn `Load Info`
  (params (`Save Game` :type "/Game/Blueprints/BP_Player_Save_Game Object Reference"))
  (set `self.Music` (`/Game/Blueprints/BP_Player_Save_Game.Music` `Save Game`))
  (set `self.Narrative` (`/Game/Blueprints/BP_Player_Save_Game.Narrative` `Save Game`))
  (`GameplayStatics.SetSoundMixClassOverride` "/Game/Assets/UI/Narrative.Narrative" "/Engine/EngineSounds/Voice.Voice" (`self.Narrative`) 1.0 0.0)
  (`GameplayStatics.PushSoundMixModifier` "/Game/Assets/UI/Narrative.Narrative")
  (`GameplayStatics.SetSoundMixClassOverride` "/Game/Assets/UI/Music.Music" "/Engine/EngineSounds/Music.Music" (`self.Music`) 1.0 0.0)
  (`GameplayStatics.PushSoundMixModifier` "/Game/Assets/UI/Music.Music"))

(fn `Save_Info`
  (params (`Save Game` :type "/Game/Blueprints/BP_Player_Save_Game Object Reference"))
  (set `/Game/Blueprints/BP_Player_Save_Game.Music` (`self.Music`) `Save Game`)
  (set `/Game/Blueprints/BP_Player_Save_Game.Narrative` (`self.Narrative`) `Save Game`))

(fn `UserConstructionScript`)